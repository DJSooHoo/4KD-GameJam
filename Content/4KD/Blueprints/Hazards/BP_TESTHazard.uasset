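; BP_TESTHazard is a test hazard Blueprint that damages the character passed to its Activate function.
; Activate applies a small fixed amount of damage with itself as the causer, then calls the parent implementation.
; The construction script runs the parent's setup, then sets the Cone's Color material parameter to black.
; The event graph holds only disabled default events.
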(fn `Activate`
  (params (Character :type "/Game/4KD/Blueprints/Characters/BP_ThirdPersonCharacter Object Reference"))
  (`GameplayStatics.ApplyDamage` Character 2.0 null self)
  (`parent.Activate` null))

(fn `UserConstructionScript`
  (`parent.UserConstructionScript`)
  (`MeshComponent.SetVectorParameterValueOnMaterials` (`self.Cone`) "Color" (0.0 0.0 0.0)))