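; BP_Projectile is a hazard projectile that damages actors it overlaps.
; On overlap, it skips its Instigator and actors that cannot be damaged, applies damage credited to the Instigator's controller, then destroys itself.
; It also destroys itself on any hit or when a short lifetime delay started in BeginPlay runs out.
; The construction script tints the Sphere red through a material Color parameter.
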(event `self.ReceiveActorBeginOverlap`
  (params (OtherActor :type "Actor Object Reference"))
  ;[1 0.3542 0.3542] Checking if target is either, the person attacking, or if the target being attacked can be hurt. If true, it will damage the target. If false, nothing will happen.
  (if (and (!= OtherActor (`self.Instigator`)) (`Actor.bCanBeDamaged` OtherActor))
    ;[0.3873 0.4415 1] Applies the damage, also destroys the projectile after damaging the target.
    (`GameplayStatics.ApplyDamage` OtherActor 1.0 (`self.GetInstigatorController`) self)
    (`self.K2_DestroyActor`)))

(event `self.ReceiveHit`
  (params (MyComp :type "PrimitiveComponent Object Reference") (Other :type "Actor Object Reference") (OtherComp :type "PrimitiveComponent Object Reference") (bSelfMoved :type Boolean) (HitLocation :type "Vector Structure") (HitNormal :type "Vector Structure") (NormalImpulse :type "Vector Structure") (Hit :type "HitResult Structure (by ref)"))
  ;[0.3604 1 0.605] Destroys projectile if it hits something.
  (`self.K2_DestroyActor`))

(event `self.ReceiveBeginPlay`
  (`KismetSystemLibrary.Delay` 6.0)
  (`self.K2_DestroyActor`))

(fn `UserConstructionScript`
  (`MeshComponent.SetVectorParameterValueOnMaterials` (`self.Sphere`) "Color" (1.0 0.0 0.0)))