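; Test cube actor that shows its health as a material color and destroys itself on death.
; On BeginPlay it hooks into its BPHealth component's death and hurt events, with death calling DestroyActor, and sets the initial color.
; UpdateHealthColor lerps the cube materials' Color parameter from black to white by the current health ratio.
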(event `self.ReceiveBeginPlay`
  (add `/Game/4KD/Blueprints/Characters/BP_Health.OnDeath` (`self.BP_Health`) (delegate `CubeDeath`))
  (`self.UpdateHealthColor`)
  (add `/Game/4KD/Blueprints/Characters/BP_Health.OnHurt` (`self.BP_Health`) (`|CreateDelegate` :!event `UpdateHealthColor`)))

(event `CubeDeath`
  (`self.K2_DestroyActor`))

(fn `UpdateHealthColor`
  (`MeshComponent.SetVectorParameterValueOnMaterials` (`self.Cube`) "Color" (`KismetMathLibrary.Conv_LinearColorToVector` (`KismetMathLibrary.LinearColorLerp` (struct) (struct :`R` 1.0 :`G` 1.0 :`B` 1.0 :`A` 1.0) (`/Game/4KD/Blueprints/Characters/BP_Health.Get Health Ratio` (`self.BP_Health`))))))

(fn `UserConstructionScript`)