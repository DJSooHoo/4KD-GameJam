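; BP_HealthPickUp is a pickup that restores a character's health to a maximum value when activated.
; The construction script tints its cube bright green through a material vector parameter.
; Its Activate override sets the character's BPHealth current health, refreshes the character's health color, prints the new value, then calls the parent Activate.
; The event graph holds only disabled default events.
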(fn `Activate`
  (params (Character :type "/Game/4KD/Blueprints/Characters/BP_ThirdPersonCharacter Object Reference"))
  (bind _bp_health (`/Game/4KD/Blueprints/Characters/BP_ThirdPersonCharacter.BP_Health` Character))
  (set `/Game/4KD/Blueprints/Characters/BP_Health.CurrentHealth` (`/Game/4KD/Blueprints/Characters/BP_Health.MaxHealth` (`self.BP_Health`)) _bp_health)
  (`/Game/4KD/Blueprints/Characters/BP_ThirdPersonCharacter.UpdateHealthColor` Character)
  (`KismetSystemLibrary.PrintString` (`KismetStringLibrary.Conv_DoubleToString` (`/Game/4KD/Blueprints/Characters/BP_Health.CurrentHealth` _bp_health)))
  (`parent.Activate` null))

(fn `UserConstructionScript`
  (`parent.UserConstructionScript`)
  (`MeshComponent.SetVectorParameterValueOnMaterials` (`self.Cube`) "Color" (`KismetMathLibrary.Conv_LinearColorToVector` (struct :`R` 0.120817 :`G` 1.0 :`A` 1.0))))