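; BP_TestMoneyPickUp is a test pickup actor that gives money to the player character on overlap.
; Its own BPCurrency component is set to a fixed amount on BeginPlay and serves as the pickup's value.
; When a BP_ThirdPersonCharacter overlaps it, it plays a click sound, passes that value to the character's BPCurrency through GainMoney, and destroys itself.
; The construction script tints the cube yellow through a material Color parameter.
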(event `self.ReceiveBeginPlay`
  (bind _output_get (set `/Game/4KD/Blueprints/Characters/BP_Currency.CurrentMoney` 33 (`self.BP_Currency`))))

(event `self.ReceiveActorBeginOverlap`
  (params (OtherActor :type "Actor Object Reference"))
  (bind _asbp_third_person_character (cast `/Game/4KD/Blueprints/Characters/BP_ThirdPersonCharacter` OtherActor))
  (`GameplayStatics.PlaySound2D` "/Engine/VREditor/Sounds/UI/Click_on_Button_Cue.Click_on_Button_Cue" 1.0 1.0 0.0 null null)
  (`/Game/4KD/Blueprints/Characters/BP_Currency.GainMoney` (`/Game/4KD/Blueprints/Characters/BP_ThirdPersonCharacter.BP_Currency` _asbp_third_person_character) (stale `self.ReceiveBeginPlay` _output_get))
  (`self.K2_DestroyActor`))

(fn `UserConstructionScript`
  (`MeshComponent.SetVectorParameterValueOnMaterials` (`self.Cube`) "Color" (1.0 1.0 0.0)))