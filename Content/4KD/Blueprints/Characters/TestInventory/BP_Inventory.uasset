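; BP_Inventory is a test inventory Blueprint that stores item quantities by name in a map.
; AddToInventory adds the incoming quantity to any existing entry for that item, or creates a new entry.
; The Inventory input action toggles an open flag and only prints a debug message, with no UI shown.
; RemoveFromInventory and SwapWithInventory are empty stubs.
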(event `InputAction|Inventory`
  (params (Key :type "Key Structure"))
  (:`Pressed`
    (if (`self.InventoryIsOpen?`)
      (`KismetSystemLibrary.PrintString` "Closing inventory." true true (struct :`R` 0.323143 :`G` 0.144128 :`B` 0.004025 :`A` 1.0))
      (set `self.InventoryIsOpen?` false)
      (else
        (set `self.InventoryIsOpen?` true)
        (`KismetSystemLibrary.PrintString` "Inventory is open." true true (struct :`R` 0.322917 :`G` 0.143765 :`B` 0.004002 :`A` 1.0))))))

(fn `AddToInventory`
  (params (`Item Name` :type Name) (Quantity :type Integer))
  (bind _inventorycontent (`self.InventoryContent`))
  (bind (_value _returnvalue) (`BlueprintMapLibrary.Map_Find` _inventorycontent `Item Name`))
  (`BlueprintMapLibrary.Map_Add` _inventorycontent `Item Name` (`KismetMathLibrary.SelectInt` (+ Quantity _value) (`local.Quantity`) _returnvalue)))

(fn `RemoveFromInventory`)

(fn `SwapWithInventory`)