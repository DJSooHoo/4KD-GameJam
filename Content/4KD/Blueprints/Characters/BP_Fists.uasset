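; BP_Fists is the player's unarmed melee weapon, with two fist components attached to the character's left and right hand sockets.
; StartAttack uses a 0.01-second timer to repeatedly sphere-trace for pawns at each fist until StopAttack clears it.
; New hit actors receive point damage, set through SendAttackDamagetoWeapon, and an impact particle message.
; An already-damaged list prevents repeat hits within a swing and is emptied by StopAttack.
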(event `/Game/4KD/Blueprints/Characters/I_WeaponInterface.SendAttackDamageToWeapon`
  (params (AttackDamage :type Integer))
  (set `self.WeaponOutputDamage` (`KismetMathLibrary.Conv_IntToDouble` AttackDamage)))

(event `AttachToPlayer`
  (bind _mesh (`Character.Mesh` (cast `/Game/4KD/Blueprints/Characters/BP_ThirdPersonCharacter` (`GameplayStatics.GetPlayerCharacter` 0) :!pure true)))
  (`SceneComponent.K2_AttachToComponent` (`self.Fist1Ref`) _mesh "hand_l" "SnapToTarget" "SnapToTarget" "KeepRelative" true)
  (`SceneComponent.K2_AttachToComponent` (`self.Fist2Ref`) _mesh "hand_r" "SnapToTarget" "SnapToTarget" "KeepRelative" true))

(event `/Game/4KD/Blueprints/Characters/I_WeaponInterface.StopAttack`
  (`KismetSystemLibrary.K2_ClearAndInvalidateTimerHandle` (stale `/Game/4KD/Blueprints/Characters/I_WeaponInterface.StartAttack` _returnvalue))
  (`KismetArrayLibrary.Array_Clear` (`self.AlreadyDamagedEnemy`)))

(event `/Game/4KD/Blueprints/Characters/I_WeaponInterface.StartAttack`
  (bind _fist2ref (`self.Fist2Ref`))
  (bind _fist1ref (`self.Fist1Ref`))
  (bind _returnvalue (`KismetSystemLibrary.K2_SetTimerDelegate` (delegate `/Game/4KD/Blueprints/Characters/I_WeaponInterface.StartAttack`) 0.01 true))
  (`|ExecutionSequence`
    (:`then_0`
      (bind _outhit (`KismetSystemLibrary.SphereTraceSingleForObjects` (`SceneComponent.K2_GetComponentLocation` _fist1ref) (`SceneComponent.K2_GetComponentLocation` _fist1ref) 30.0 (`|MakeArray` "ObjectTypeQuery3" :!type "EObjectTypeQuery Enum") false (`|MakeArray` (cast `/Game/4KD/Blueprints/Characters/BP_ThirdPersonCharacter` (`GameplayStatics.GetPlayerCharacter` 0) :!pure true) :!type "Actor Object Reference")))
      (bind (_bblockinghit _binitialoverlap _time _distance _location _impactpoint _normal _impactnormal _physmat _hitactor) (`GameplayStatics.BreakHitResult` _outhit))
      (if (not (`KismetArrayLibrary.Array_Contains` (`self.AlreadyDamagedEnemy`) _hitactor))
        (`KismetArrayLibrary.Array_Add` (`self.AlreadyDamagedEnemy`) _hitactor)
        (message `/Game/4KD/Blueprints/Characters/I_Character.PassWeaponParticleSystem` _hitactor "/Game/FlexibleCombatSystem/DemoRoom/VFX/P_FistsImpact.P_FistsImpact")
        (`GameplayStatics.ApplyPointDamage` _hitactor (`self.WeaponOutputDamage`) _impactpoint _outhit null (cast `/Game/4KD/Blueprints/Characters/BP_ThirdPersonCharacter` (`GameplayStatics.GetPlayerCharacter` 0) :!pure true))))
    (:`then_1`
      (bind _outhit_2 (`KismetSystemLibrary.SphereTraceSingleForObjects` (`SceneComponent.K2_GetComponentLocation` _fist2ref) (`SceneComponent.K2_GetComponentLocation` _fist2ref) 50.0 (`|MakeArray` "ObjectTypeQuery3" :!type "EObjectTypeQuery Enum") false (`|MakeArray` (cast `/Game/4KD/Blueprints/Characters/BP_ThirdPersonCharacter` (`GameplayStatics.GetPlayerCharacter` 0) :!pure true) :!type "Actor Object Reference")))
      (bind (_bblockinghit_2 _binitialoverlap_2 _time_2 _distance_2 _location_2 _impactpoint_2 _normal_2 _impactnormal_2 _physmat_2 _hitactor_2) (`GameplayStatics.BreakHitResult` _outhit_2))
      (if (not (`KismetArrayLibrary.Array_Contains` (`self.AlreadyDamagedEnemy`) _hitactor_2))
        (`KismetArrayLibrary.Array_Add` (`self.AlreadyDamagedEnemy`) _hitactor_2)
        (message `/Game/4KD/Blueprints/Characters/I_Character.PassWeaponParticleSystem` _hitactor_2 "/Game/FlexibleCombatSystem/DemoRoom/VFX/P_FistsImpact.P_FistsImpact")
        (`GameplayStatics.ApplyPointDamage` _hitactor_2 (`self.WeaponOutputDamage`) _impactpoint_2 _outhit_2 null (cast `/Game/4KD/Blueprints/Characters/BP_ThirdPersonCharacter` (`GameplayStatics.GetPlayerCharacter` 0) :!pure true))))))

(fn `UserConstructionScript`)