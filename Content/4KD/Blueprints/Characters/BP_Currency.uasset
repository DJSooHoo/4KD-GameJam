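; Currency Blueprint that tracks money for characters, with gain and spend events for the player and a drop event for NPCs.
; Gains clamp at a maximum, and purchases are refused when funds are short, each reported by printed messages.
; Dropping only subtracts the balance captured at BeginPlay, without spawning anything.
; A test key prints the current balance.
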(event `self.ReceiveBeginPlay`
  ;[1 1 1] Setting Droppable Money to Current Money
  (set `self.DroppableMoney` (`self.CurrentMoney`)))

(event `GainMoney`
  (params (IncomingMoney :type Integer))
  ;[0.191 0.2518 1] Event to handle gaining money (Player specific)
  (`self.FullOfMoney?` IncomingMoney))

(event `SpendingMoney`
  (params (Cost :type Integer))
  ;[0.2531 0.3765 1] Event to handle spending money (Player specific)
  (`self.Buying` Cost))

(event `DropMoney`
  ;[1 0.3529 0.2531] Event to handle dropping money (NPC specific)
  (`self.Dropping Money`))

(event `Key|M`
  (params (Key :type "Key Structure"))
  ;[0 0 0] TESTING: Input to check if money is being working correctly.
  (:`Pressed`
    (`KismetSystemLibrary.PrintString` (`KismetStringLibrary.Concat_StrStr` "I have " "$" (`KismetStringLibrary.Conv_IntToString` (`self.CurrentMoney`)) "."))))

(fn `AddMoney`
  (params (IncomingMoney :type Integer))
  (set `self.CurrentMoney` (+ IncomingMoney (`self.CurrentMoney`))))

(fn `Buying`
  (params (Cost :type Integer))
  (if (> Cost (`self.CurrentMoney`))
    (`KismetSystemLibrary.PrintString` "I don't have enough money..." true true (struct :`G` 1.0 :`B` 0.0425 :`A` 1.0) 5.0)
    (else
      (`self.Losing Money` Cost))))

(fn `Dropping Money`
  (`self.Losing Money` (`self.DroppableMoney`)))

(fn `FullOfMoney?`
  (params (IncomingMoney :type Integer))
  (if (== (`self.CurrentMoney`) (`self.MaxMoney`))
    (`KismetSystemLibrary.PrintString` "I can't carry any more money..." true true (struct :`R` 0.237298 :`G` 1.0 :`A` 1.0) 5.0)
    (elif (>= (+ IncomingMoney (`self.CurrentMoney`)) (`self.MaxMoney`))
      (set `self.CurrentMoney` (`self.MaxMoney`))
      (`KismetSystemLibrary.PrintString` "I can't carry any more money..." true true (struct :`R` 0.237298 :`G` 1.0 :`A` 1.0) 5.0)
      (else
        (`self.AddMoney` IncomingMoney)))))

(fn `Losing Money`
  (params (DepartingMoney :type Integer))
  (set `self.CurrentMoney` (- (`self.CurrentMoney`) DepartingMoney)))