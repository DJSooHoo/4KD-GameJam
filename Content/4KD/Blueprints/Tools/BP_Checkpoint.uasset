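; BP_Checkpoint is a placeable trigger that records player progress when the third-person character overlaps it.
; On overlap it writes its Index into the character's CurrentCheckpoint, so re-entering an earlier checkpoint overwrites the value.
; On first trigger only, it has the BaseMap streaming level's script show a checkpoint message with its flavor text and designer name.
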(event `self.ReceiveActorBeginOverlap`
  (params (OtherActor :type "Actor Object Reference"))
  (bind _asbp_third_person_character (cast `/Game/4KD/Blueprints/Characters/BP_ThirdPersonCharacter` OtherActor))
  (set `/Game/4KD/Blueprints/Characters/BP_ThirdPersonCharacter.CurrentCheckpoint` (`self.Index`) _asbp_third_person_character)
  (if (not (`self.Triggered`))
    (set `self.Triggered` true)
    (message `/Game/4KD/Blueprints/Characters/I_Checkpoint.ShowCheckpoint` (`GameplayStatics.GetStreamingLevel` "BaseMap") (`self.Checkpoint Flavor Text`) (`self.Designer Name`))))

(fn `UserConstructionScript`)