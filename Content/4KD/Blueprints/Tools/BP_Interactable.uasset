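; Base interactable with an overlap volume that lets the player trigger an action via a "Press E" prompt.
; Overlap shows controller UI text built by BuildCTAString, which also checks for an optional required collectible.
; If satisfied, it binds to the controller's OnInteract, then fires its own OnInteract dispatcher when triggered.
; Repeatable interactions re-arm after a cooldown, and enable/disable events toggle availability and collision.
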(event `self.ReceiveActorBeginOverlap`
  (params (OtherActor :type "Actor Object Reference"))
  (bind _thirdpersoncontroller (`self.ThirdPersonController`))
  (bind _asbp_third_person_controller (cast `/Game/4KD/Blueprints/Characters/BP_ThirdPersonController` OtherActor))
  (set `self.ThirdPersonController` _asbp_third_person_controller)
  ;[1 1 1] Is Overlapped Actor, the player?
  (if (== OtherActor (`GameplayStatics.GetPlayerPawn` 0))
    (bind _asbp_third_person_character (cast `/Game/4KD/Blueprints/Characters/BP_ThirdPersonCharacter` OtherActor))
    (set `self.Player` _asbp_third_person_character)
    ;[1 1 1] Can the player interact with this?
    (if (`self.canInteract`)
      ;[1 1 1] Show UI Feedback
      (`/Game/4KD/Blueprints/Characters/BP_ThirdPersonController.Display UI Input Message` _thirdpersoncontroller)
      (bind _returnvalue (`self.Build CTA String`))
      (`/Game/4KD/Blueprints/Characters/BP_ThirdPersonController.Change UI Input Message` _thirdpersoncontroller _returnvalue)
      ;[1 1 1] Has Required Object?
      (if (`self.hasRequiredObject`)
        ;[1 1 1] Bind OnInteract
        (add `/Game/4KD/Blueprints/Characters/BP_ThirdPersonController.OnInteract` (`self.ThirdPersonController`) (delegate `Event OnInteract`))
        (set `self.isHere` true)))))

(event `Event OnInteract`
  (bind _thirdpersoncontroller (`self.ThirdPersonController`))
  ;[1 1 1] Is the player here AND can interact?
  (if (and (`self.isHere`) (`self.canInteract`))
    (set `self.canInteract` false)
    ;[1 1 1] Hide the UI Feedback
    (`/Game/4KD/Blueprints/Characters/BP_ThirdPersonController.Hide UI Input Message` (`self.ThirdPersonController`))
    (`self.OnInteract`)
    ;[1 1 1] Reset if it is repeatable
    (if (`self.isRepeatable`)
      (`KismetSystemLibrary.Delay` (`self.repeatCooldown`))
      (set `self.canInteract` true)
      ;[1 1 1] Check if player is still in the overlap volume
      (if (> (`KismetArrayLibrary.Array_Length` (`PrimitiveComponent.GetOverlappingActors` (`self.OverlapVolume`) "/Game/4KD/Blueprints/Characters/BP_ThirdPersonCharacter.BP_ThirdPersonCharacter_C")) 0)
        ;[1 1 1] Show UI Feedback
        (`/Game/4KD/Blueprints/Characters/BP_ThirdPersonController.Display UI Input Message` _thirdpersoncontroller)
        (bind _returnvalue (`self.Build CTA String`))
        (`/Game/4KD/Blueprints/Characters/BP_ThirdPersonController.Change UI Input Message` _thirdpersoncontroller _returnvalue)))))

(event `self.ReceiveActorEndOverlap`
  (params (OtherActor :type "Actor Object Reference"))
  (bind _asbp_third_person_controller (cast `/Game/4KD/Blueprints/Characters/BP_ThirdPersonController` OtherActor))
  (clear `/Game/4KD/Blueprints/Characters/BP_ThirdPersonController.OnInteract` _asbp_third_person_controller)
  (set `self.isHere` false)
  (`/Game/4KD/Blueprints/Characters/BP_ThirdPersonController.Hide UI Input Message` _asbp_third_person_controller))

(event `DisableInteraction`
  (set `self.canInteract` false)
  (`PrimitiveComponent.SetCollisionEnabled` (`self.OverlapVolume`) "NoCollision")
  (bind _thirdpersoncontroller (`self.ThirdPersonController`)
    (:`then`
      (clear `/Game/4KD/Blueprints/Characters/BP_ThirdPersonController.OnInteract` _thirdpersoncontroller)
      (`/Game/4KD/Blueprints/Characters/BP_ThirdPersonController.Hide UI Input Message` _thirdpersoncontroller))
    (:`else`)))

(event `EnableInteraction`
  (set `self.canInteract` true)
  (`PrimitiveComponent.SetCollisionEnabled` (`self.OverlapVolume`) "QueryAndPhysics"))

(fn `Build CTA String`
  (returns (ReturnValue :type String))
  (bind _requiredcollectible (`self.RequiredCollectible`))
  (`/Engine/EditorBlueprintResources/StandardMacros.IsValid` (`self.RequiredCollectible`)
    (:`Is Valid`
      (bind _found (`/Game/4KD/Blueprints/Characters/BP_ThirdPersonController.Check for Collectible` (`self.ThirdPersonController`) _requiredcollectible))
      (bind _output_get (set `self.hasRequiredObject` _found))
      (if _output_get
        (return (`KismetStringLibrary.Concat_StrStr` "Press E to " (`KismetStringLibrary.ToUpper` (`self.Interact Action`)) " with " (`/Game/4KD/Blueprints/Tools/BP_Collectible.UIObjectName` (`self.RequiredCollectible`))))
        (else
          (return (`KismetStringLibrary.Concat_StrStr` (`/Game/4KD/Blueprints/Tools/BP_Collectible.UIObjectName` _requiredcollectible) "Required")))))
    (:`Is Not Valid`
      (set `self.hasRequiredObject` true)
      (return (`KismetStringLibrary.Concat_StrStr` "Press E to " (`KismetStringLibrary.ToUpper` (`self.Interact Action`)))))))

(fn `UserConstructionScript`)