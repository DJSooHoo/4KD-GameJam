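; BP_Collectible is a world item the third-person player collects through an interact prompt.
; On overlap it checks CanInteract, then binds to the character's OnInteract and shows a "Press E to Collect" prompt with its name.
; Interacting plays a sound, passes itself to the pawn's CollectMessage, disables mesh collision and blocks reuse.
; Leaving unbinds and hides the prompt, while SetCanInteract can enable collection during an overlap.
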(event `self.ReceiveActorBeginOverlap`
  (params (OtherActor :type "Actor Object Reference"))
  (bind _asbp_third_person_character (cast `/Game/4KD/Blueprints/Characters/BP_ThirdPersonCharacter` OtherActor))
  (set `self.Player` _asbp_third_person_character)
  (bind _asbp_third_person_controller (cast `/Game/4KD/Blueprints/Characters/BP_ThirdPersonController` OtherActor))
  (set `self.PlayerController` _asbp_third_person_controller)
  (set `self.isHere` true)
  (`self.Check for Can Interact` (delegate `Event OnInteract`)))

(event `Event OnInteract`
  (if (and (`self.isHere`) (`self.canInteract`))
    (set `self.canInteract` false)
    (`/Game/4KD/Blueprints/Characters/BP_ThirdPersonController.Hide UI Input Message` (`self.PlayerController`))
    (`GameplayStatics.PlaySound2D` "/Engine/VREditor/Sounds/UI/Flashlight_Switch.Flashlight_Switch" 1.0 1.0 0.0 null null)
    (message `/Game/4KD/Blueprints/Characters/I_Collect.Collect` (`GameplayStatics.GetPlayerPawn` 0) self)
    (`self.SetActorHiddenInGame` self false)
    (`PrimitiveComponent.SetCollisionEnabled` (`self.ObjectMesh`) "NoCollision")
    (set `self.canInteract` false)))

(event `self.ReceiveActorEndOverlap`
  (params (OtherActor :type "Actor Object Reference"))
  (bind _asbp_third_person_character (cast `/Game/4KD/Blueprints/Characters/BP_ThirdPersonCharacter` OtherActor))
  (clear `/Game/4KD/Blueprints/Characters/BP_ThirdPersonCharacter.OnInteract` _asbp_third_person_character)
  (set `self.isHere` false)
  (`/Game/4KD/Blueprints/Characters/BP_ThirdPersonCharacter.Hide UI Input Message` _asbp_third_person_character))

(event `SetCanInteract`
  (params (canInteract :type Boolean))
  (set `self.canInteract` canInteract)
  (if (`self.isHere`)
    (`self.Check for Can Interact` (delegate `Event OnInteract`))))

(fn `Check for Can Interact`
  (params (Delegate :type "Object Object Reference (by ref)"))
  (bind _player (`self.Player`))
  (if (`self.canInteract`)
    (add `/Game/4KD/Blueprints/Characters/BP_ThirdPersonCharacter.OnInteract` _player Delegate)
    (`/Game/4KD/Blueprints/Characters/BP_ThirdPersonCharacter.Display UI Input Message` _player)
    (`/Game/4KD/Blueprints/Characters/BP_ThirdPersonCharacter.Change UI Input Message` _player (`KismetStringLibrary.Concat_StrStr` "Press E to Collect " (`self.UIObjectName`)))))

(fn `UserConstructionScript`)